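; Gameplay ability for the third light attack in a combo chain, which commits and plays an attack montage.
; Two parallel gameplay event waits track the combo window: opening swaps the Combo2 window tag for the general combo window tag on the avatar, with replication.
; The window end event removes that tag and ends the ability, as does montage completion, interruption or cancellation, though these montage exits skip the tag cleanup.
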(event Ability|EventActivateAbility
  (bind _returnvalue (Ability|GetAvatarActorfromActorInfo))
  (Ability|CommitAbility)
  (|PlayMontageandWaitProxy "None" (Variables|Default|GetMontage%20to%20Play) 1.0 "None" true 1.0 0.0 false
    (:then
      (Ability|Tasks|WaitGameplayEvent "(TagName=\"Event.ComboWindowOpen\")" 0
        (:then
          (Ability|Tasks|WaitGameplayEvent "(TagName=\"Event.ComboWindowEnd\")" 0
            (:EventReceived
              (Ability|GameplayEffect|RemoveLooseGameplayTags (Ability|GetAvatarActorfromActorInfo) (Variables|Default|GetComboWindowTag) true)
              (Ability|EndAbility))))
        (:EventReceived
          (Ability|GameplayEffect|RemoveLooseGameplayTags _returnvalue (Variables|Default|GetCombo2WindowTag) true)
          (Ability|GameplayEffect|AddLooseGameplayTags _returnvalue (Variables|Default|GetComboWindowTag) true))))
    (:OnCompleted
      (Ability|EndAbility :!label _label))
    (:OnInterrupted
      (goto _label))
    (:OnCancelled
      (goto _label))))

(event Ability|EventOnEndAbility
  (params (bWasCancelled :type Boolean)))